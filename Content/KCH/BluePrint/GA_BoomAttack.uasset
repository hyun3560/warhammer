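; GA_BoomAttack is a gameplay ability that makes an explosion attack centered on its owning actor.
; On activation it spawns the explosion particle effect at the owner's location and a BP_HitBox at the owner's transform, with that actor as owner.
; The hit box runs a zero-distance box trace that is passed the ability's Damage value, then the ability ends immediately.
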(event `self.K2_ActivateAbility`
  (bind _returnvalue (`self.GetOwningActorFromActorInfo`))
  (`parent.K2_ActivateAbility`)
  (`GameplayStatics.SpawnEmitterAtLocation` "/Game/StarterContent/Particles/P_Explosion.P_Explosion" (`Actor.K2_GetActorLocation` (`self.GetOwningActorFromActorInfo`)))
  (bind _returnvalue_2 (`|SpawnActorFromClass` "/Game/KCH/BluePrint/BP_HitBox.BP_HitBox_C" (`Actor.GetTransform` _returnvalue) "Undefined" "MultiplyWithRoot" _returnvalue (0.0 0.0 0.0) (struct) 0.0 10.0 (`Actor.Instigator` _returnvalue)))
  (`Hit_Box.BoxTraceHit` _returnvalue_2 0.0 (200.0 200.0 200.0) (`self.Damage`))
  (`self.K2_EndAbility`))

(event `self.K2_OnEndAbility`
  (params (bWasCancelled :type Boolean))
  (`parent.K2_OnEndAbility` bWasCancelled))