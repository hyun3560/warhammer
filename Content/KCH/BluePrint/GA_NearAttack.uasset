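; GA_NearAttack is a gameplay ability that performs a melee hit in front of its owner.
; On activation it waits once for the AnimEvent gameplay event on the owning actor.
; When the event arrives, it spawns a BP_HitBox at the owner's transform and calls its box trace with a fixed range, size and the ability's Damage.
; The graph itself never calls EndAbility.
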(event `self.K2_ActivateAbility`
  (bind _returnvalue (`self.GetOwningActorFromActorInfo`))
  (bind _returnvalue_2 (`self.GetOwningActorFromActorInfo`))
  (`parent.K2_ActivateAbility`)
  (`AbilityAsync_WaitGameplayEvent.WaitGameplayEventToActor` _returnvalue (struct :`TagName` "AnimEvent") true
    (:`EventReceived`
      (bind _returnvalue_3 (`|SpawnActorFromClass` "/Game/KCH/BluePrint/BP_HitBox.BP_HitBox_C" (`Actor.GetTransform` _returnvalue) "Undefined" "MultiplyWithRoot" _returnvalue_2 (0.0 0.0 0.0) (struct) 0.0 10.0 (`Actor.Instigator` _returnvalue_2)))
      (`Hit_Box.BoxTraceHit` _returnvalue_3 200.0 (100.0 100.0 100.0) (`self.Damage`)))))