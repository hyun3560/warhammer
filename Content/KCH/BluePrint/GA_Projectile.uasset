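; Gameplay ability that lets an AI-controlled owner fire a projectile at its blackboard target.
; After parent activation, it waits for a single AnimEvent gameplay event on the owner, then continues only on the authority.
; It spawns a BP_HitBox_Projectile just ahead of the owner.
; It then casts the blackboard "Target" to BP_ThirdPersonCharacter and launches the projectile toward that character's current location.
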(event `self.K2_ActivateAbility`
  (bind _returnvalue (`self.GetOwningActorFromActorInfo`))
  (`parent.K2_ActivateAbility`)
  (`AbilityAsync_WaitGameplayEvent.WaitGameplayEventToActor` _returnvalue (struct :`TagName` "AnimEvent") true
    (:`EventReceived`
      (`self.K2_HasAuthority`
        (:`True`
          (bind _returnvalue_2 (`|SpawnActorFromClass` "/Game/KCH/BluePrint/BP_HitBox_Projectile.BP_HitBox_Projectile_C" (`KismetMathLibrary.MakeTransform` (+ (`Actor.K2_GetActorLocation` _returnvalue) (* (`Actor.GetActorForwardVector` _returnvalue) 100.0))) "Undefined" "MultiplyWithRoot" _returnvalue null))
          (bind _asbp_third_person_character (cast `/Game/ThirdPerson/Blueprints/BP_ThirdPersonCharacter` (`BlackboardComponent.GetValueAsObject` (`AIBlueprintHelperLibrary.GetBlackboard` (`self.GetOwningActorFromActorInfo`)) "Target")))
          (`HitBox_Projectile.LaunchToTarget` _returnvalue_2 (`Actor.K2_GetActorLocation` _asbp_third_person_character)))))))

(event `self.K2_OnEndAbility`
  (params (bWasCancelled :type Boolean)))