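; GA_BaseMonsterAttack is a Gameplay Ability that plays an enemy's attack montage on its owning BP_BaseEnemy.
; On activation it first stores a Damage value by looping through DT_MonterData rows for the one whose ID matches the enemy's UniqueID.
; It then plays the enemy's AttackMontage and ends the ability on blend out, interruption or cancel.
; Damage is only set here, not applied.
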(event `self.K2_ActivateAbility`
  (bind _asbp_base_enemy (cast `/Game/KCH/BluePrint/BP_BaseEnemy` (`self.GetOwningActorFromActorInfo`)))
  (set `self.As BP Base Enemy` _asbp_base_enemy)
  (`self.Set Damage`)
  (`AbilityTask_PlayMontageAndWait.CreatePlayMontageAndWaitProxy` "None" (`BaseEnemyCharacter.AttackMontage` _asbp_base_enemy)
    (:`OnBlendOut`
      _)
    (:`OnInterrupted`
      _)
    (:`OnCancelled`
      _))
  (`self.K2_EndAbility`))

(event `Set Damage`
  (bind _outrownames (`DataTableFunctionLibrary.GetDataTableRowNames` "/Game/KCH/DataTable/DT_MonterData.DT_MonterData"))
  (for _array_element _outrownames
    (bind _returnvalue (`|GetDataTableRow` "/Game/KCH/DataTable/DT_MonterData.DT_MonterData" _array_element)
      (:`then`
        (if (== (break `EnemyTableRow` _returnvalue) (`BaseEnemyCharacter.UniqueID` (`self.As BP Base Enemy`)))
          (set `self.Damage` (`.Damage` (break `EnemyTableRow` _returnvalue)))
          (break))))))