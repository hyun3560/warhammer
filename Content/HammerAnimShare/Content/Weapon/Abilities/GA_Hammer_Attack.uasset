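; GA_Hammer_Attack is the hammer weapon's attack ability, supplying its primary melee combo swing.
; ExecutePrimaryAttack casts the avatar to the Murdock player and forwards combo input to that character's WeaponComponent, ignoring the passed-in component and always returning true.
; The component receives linked first-person arms and third-person body anim instances, their swing montages and shared combo section names.
; ActivateAbility only prints a debug string and ends immediately.
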(event `self.K2_ActivateAbility`
  (`KismetSystemLibrary.PrintString` "hammer")
  (`self.K2_EndAbility`))

(fn `ExecutePrimaryAttack`
  (params (WeaponComponent :type "LMSWeaponComponent Object Reference"))
  (returns (ReturnValue :type Boolean))
  (bind _asbp_murdock_player_character (cast `/Game/ThirdPerson/Blueprints/BP_MurdockPlayerCharacter` (`self.GetAvatarActorFromActorInfo`))
    (:`then`
      (`LMSWeaponComponent.HandleMeleeComboInputLinked` (`LMS_TeamProjectCharacter.WeaponComponent` _asbp_murdock_player_character) (`SkeletalMeshComponent.GetAnimInstance` (`/Game/ThirdPerson/Blueprints/BP_MurdockPlayerCharacter.SK_Murdock_FP_Arms` _asbp_murdock_player_character)) "/Game/_LocalOnly/Animations/hammer_swing_Montage.hammer_swing_Montage" (`SkeletalMeshComponent.GetAnimInstance` (`Character.Mesh` _asbp_murdock_player_character)) "/Game/_LocalOnly/Animations/Hammer_Swing_3P_Montage.Hammer_Swing_3P_Montage" (`self.Combo Section Names`)))
    (:`CastFailed`
      _))
  (return true))