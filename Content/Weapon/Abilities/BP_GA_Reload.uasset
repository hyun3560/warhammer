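; Gameplay ability that plays rifle reload animations for the Murdock player character.
; PlayReloadMontage casts the avatar, plays the first-person montage on the arms mesh, has the WeaponComponent play the replicated third-person montage, then ends the ability immediately without waiting for either montage.
; A separate Reload function plays only the first-person montage, with a debug print.
; OnEndAbility is empty.
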(event `self.PlayReloadMontage`
  (bind _asbp_murdock_player_character (cast `/Game/ThirdPerson/Blueprints/BP_MurdockPlayerCharacter` (`self.GetAvatarActorFromActorInfo`)))
  (`AnimInstance.Montage_Play` (`SkeletalMeshComponent.GetAnimInstance` (`/Game/ThirdPerson/Blueprints/BP_MurdockPlayerCharacter.SK_Murdock_FP_Arms` _asbp_murdock_player_character)) "/Game/JJO/Rifle_Animation/First/First_Rifle_Reload_Montage.First_Rifle_Reload_Montage" 1.0 "MontageLength" 0.0 false)
  (`LMSWeaponComponent.PlayReplicatedThirdPersonWeaponMontage` (`LMS_TeamProjectCharacter.WeaponComponent` _asbp_murdock_player_character) "/Game/JJO/Rifle_Animation/Third/Third_Rifle_Reload_Montage.Third_Rifle_Reload_Montage" "None" 1.0)
  (`self.K2_EndAbility`))

(fn `Reload`
  (`KismetSystemLibrary.PrintString` "Hello")
  (bind _asbp_murdock_player_character (cast `/Game/ThirdPerson/Blueprints/BP_MurdockPlayerCharacter` (`self.GetAvatarActorFromActorInfo`)))
  ;[1 1 1] Reload
  (`AnimInstance.Montage_Play` (`SkeletalMeshComponent.GetAnimInstance` (`/Game/ThirdPerson/Blueprints/BP_MurdockPlayerCharacter.SK_Murdock_FP_Arms` _asbp_murdock_player_character)) "/Game/JJO/Rifle_Animation/First/First_Rifle_Reload_Montage.First_Rifle_Reload_Montage" 1.0 "MontageLength" 0.0 false)
  (`self.K2_EndAbility`))