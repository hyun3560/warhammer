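; Gameplay ability for the rifle's secondary (aim) action, which drives weapon montages in first and third person.
; On secondary start, it plays both montages through the WeaponComponent from their Default section, with the third-person one replicated.
; On secondary end, it blends out the first-person montage and plays the replicated third-person montage at ShootStart instead of stopping it.
; Activate and End events are empty, and older direct AnimInstance and projectile-firing logic is left disconnected.
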(event `self.OnSecondaryStarted`
  (params (WeaponComponent :type "LMSWeaponComponent Object Reference"))
  (`LMSWeaponComponent.PlayFirstPersonWeaponMontage` WeaponComponent "/Game/JJO/Rifle_Animation/First/First_TheEleven_Montage.First_TheEleven_Montage" "Default" 1.0)
  (`LMSWeaponComponent.PlayReplicatedThirdPersonWeaponMontage` WeaponComponent "/Game/JJO/Rifle_Animation/Third/Third_TheEleven_Montage1.Third_TheEleven_Montage1" "Default" 1.0))

(event `self.OnSecondaryEnded`
  (params (WeaponComponent :type "LMSWeaponComponent Object Reference") (bWasCancelled :type Boolean))
  (`LMSWeaponComponent.StopFirstPersonWeaponMontage` WeaponComponent "/Game/JJO/Rifle_Animation/First/First_TheEleven_Montage.First_TheEleven_Montage" 0.15)
  (`LMSWeaponComponent.PlayReplicatedThirdPersonWeaponMontage` WeaponComponent "/Game/JJO/Rifle_Animation/Third/Third_TheEleven_Montage1.Third_TheEleven_Montage1" "ShootStart" 1.0))