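; GA_Rifle_Fire is the gameplay ability for the rifle's primary fire.
; ExecutePrimaryAttack plays a first-person arms montage on the Murdock player character, then has the WeaponComponent consume ammo, fire a projectile and play a replicated third-person montage.
; The projectile fires regardless of the ammo check's result, and the function ends the ability and returns false.
; ActivateAbility itself only prints a debug string and ends.
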(event `self.K2_ActivateAbility`
  (`KismetSystemLibrary.PrintString` "gun")
  (`self.K2_EndAbility`))

(fn `ExecutePrimaryAttack`
  (params (WeaponComponent :type "LMSWeaponComponent Object Reference"))
  (returns (ReturnValue :type Boolean))
  (bind _asbp_murdock_player_character (cast `/Game/ThirdPerson/Blueprints/BP_MurdockPlayerCharacter` (`self.GetAvatarActorFromActorInfo`)))
  (`AnimInstance.Montage_Play` (`SkeletalMeshComponent.GetAnimInstance` (`/Game/ThirdPerson/Blueprints/BP_MurdockPlayerCharacter.SK_Murdock_FP_Arms` _asbp_murdock_player_character)) "/Game/JJO/Rifle_Animation/First/First_Rifle_Fire_Fast_Montage.First_Rifle_Fire_Fast_Montage" 1.0 "MontageLength" 0.0 false)
  (`LMSWeaponComponent.TryConsumeAmmo` WeaponComponent 1 true)
  (`LMSWeaponComponent.FireRifleProjectile` WeaponComponent 1.0)
  (`LMSWeaponComponent.PlayReplicatedThirdPersonWeaponMontage` WeaponComponent "/Game/JJO/Rifle_Animation/Third/Third_Rifle_Fire_Fast_Montage.Third_Rifle_Fire_Fast_Montage" "None" 1.0)
  (`self.K2_EndAbility`)
  (return false))