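; First-person rifle fire gameplay ability for the Murdock player character, currently an unwired stub.
; ActivateAbility, OnEndAbility and the ExecutePrimaryAttack0 function do no active work, so the ability neither plays animation nor ends itself.
; Disconnected leftover nodes show a fast-fire montage played on the character's first-person arms followed by EndAbility, plus debug prints and a stray reload montage.
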(event `self.K2_ActivateAbility`)

(fn `ExecutePrimaryAttack_0`
  (params (WeaponComponent :type "LMSWeaponComponent Object Reference"))
  (returns (ReturnValue :type Boolean)))